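; Raw iron item, by its name, that moves toward the output point of the last overlapped BP_Pipe.
; Any damage event starts a timeline through a DoOnce, easing it from its current position toward that point and matching its rotation.
; Each Tick, a small offset sphere trace ignoring pipes sets IsFrontEmty, which is true on a hit despite its name.
; A hit stops the timeline; otherwise timeline updates re-arm the DoOnce.
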(event `self.ReceiveBeginPlay`)

(event `self.ReceiveActorBeginOverlap`
  (params (OtherActor :type "Actor Object Reference"))
  (bind _asbp_pipe (cast `/Game/object_transform/BP_Pipe` OtherActor))
  (set `self.Overlapping_Pipe` _asbp_pipe))

(event `self.ReceiveAnyDamage`
  (params (Damage :type "Float (single-precision)") (DamageType :type "DamageType Object Reference") (InstigatedBy :type "Controller Object Reference") (DamageCauser :type "Actor Object Reference"))
  (bind _out_p (`/Game/object_transform/BP_Pipe.out_P` (`self.Overlapping_Pipe`)))
  (`/Engine/EditorBlueprintResources/StandardMacros.DoOnce` false :!label _label
    (:`Completed`
      (bind (_direction _newtrack_1) (`Timeline|Vector_Value` :!label _label_2)
        (:`Update`
          (set `self.First_Location` (`SceneComponent.K2_GetComponentLocation` (`self.DefaultSceneRoot`)))
          (set `self.Last_Location` (`SceneComponent.K2_GetComponentLocation` _out_p))
          (`SceneComponent.K2_SetWorldTransform` (`self.DefaultSceneRoot`) (`KismetMathLibrary.MakeTransform` (+ (`self.First_Location`) (* (* 0.5 _newtrack_1) (- (`self.Last_Location`) (`self.First_Location`)))) (`SceneComponent.K2_GetComponentRotation` _out_p)) false false)
          (if (`self.Is_Front_emty`)
            (goto _label_2 :!via `Stop`)
            (else
              (goto _label :!via `Reset`))))))))

(event `self.ReceiveTick`
  (params (DeltaSeconds :type "Float (single-precision)"))
  (bind _returnvalue (+ (`SceneComponent.K2_GetComponentLocation` (`self.Sphere`)) (-20.0 0.0 0.0)))
  (`|ExecutionSequence`
    (:`then_0`
      (bind _outactors (`GameplayStatics.GetAllActorsOfClass` "/Game/object_transform/BP_Pipe.BP_Pipe_C"))
      (bind (_outhit _returnvalue_2) (`KismetSystemLibrary.SphereTraceSingle` _returnvalue _returnvalue 10.0 "TraceTypeQuery1" false _outactors "ForOneFrame"))
      (set `self.Is_Front_emty` _returnvalue_2))
    (:`then_1`
      (`GameplayStatics.GetAllActorsOfClass` "/Game/object_transform/BP_Building_Base.BP_Building_Base_C"))))

(fn `UserConstructionScript`)
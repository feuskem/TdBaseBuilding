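; BP_Spliter is a two-output resource splitter building whose distribution logic is unfinished.
; Each Tick, debug-drawn sphere traces at Rg and Rg1 ignore BP_Pipe actors and store hits in OP1 and OP2.
; Per-resource functions spawn an item actor at a given output and decrement its stored count.
; The FlipFlop alternation and ResourceType switches that call these functions are disconnected, so nothing spawns.
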(event `self.ReceiveTick`
  (params (DeltaSeconds :type "Float (single-precision)"))
  (bind _returnvalue (`SceneComponent.K2_GetComponentLocation` (`self.rg`)))
  (bind _returnvalue_2 (`SceneComponent.K2_GetComponentLocation` (`self.rg1`)))
  (`|ExecutionSequence`
    (:`then_2`
      (bind _outactors (`GameplayStatics.GetAllActorsOfClass` "/Game/object_transform/pipes/BP_Pipe.BP_Pipe_C"))
      (bind (_outhit _returnvalue_3) (`KismetSystemLibrary.SphereTraceSingle` _returnvalue _returnvalue 20.0 "TraceTypeQuery1" false _outactors "ForOneFrame"))
      (set `self.OP1` _returnvalue_3))
    (:`then_3`
      (bind _outactors_2 (`GameplayStatics.GetAllActorsOfClass` "/Game/object_transform/pipes/BP_Pipe.BP_Pipe_C"))
      (bind (_outhit_2 _returnvalue_4) (`KismetSystemLibrary.SphereTraceSingle` _returnvalue_2 _returnvalue_2 20.0 "TraceTypeQuery1" false _outactors_2 "ForOneFrame"))
      (set `self.OP2` _returnvalue_4))))

(fn `UserConstructionScript`)
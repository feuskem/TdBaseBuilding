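; Base building actor that can spawn an actor of a given class at its OutputPoint component.
; SpawnMesh takes a count and, while it is above zero, spawns the class at that point's location and rotation and returns the count minus one.
; BeginPlay only casts the player controller to BP_collection, and Tick and the construction script do no work.
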(event `self.ReceiveBeginPlay`
  (cast `/Game/object_transform/BP_collection` (`GameplayStatics.GetPlayerController` 0)))

(event `self.ReceiveTick`
  (params (DeltaSeconds :type "Float (single-precision)"))
  (`|ExecutionSequence`))

(fn `SpawnMesh`
  (params (InputPin :type Integer64) (Class :type "Actor Class Reference"))
  (returns (OutputPin :type Integer64))
  (bind _output_point (`self.Output_Point`))
  (if (> InputPin 0)
    (`|SpawnActorFromClass` Class (`KismetMathLibrary.MakeTransform` (`SceneComponent.K2_GetComponentLocation` _output_point) (`SceneComponent.K2_GetComponentRotation` _output_point)) "Undefined" "OverrideRootScale" null null)
    (return (- InputPin 1))))

(fn `UserConstructionScript`)
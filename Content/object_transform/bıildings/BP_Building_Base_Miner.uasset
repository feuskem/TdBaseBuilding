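; Base miner building that accumulates Raw Iron, Carbon or Soil, based on ResourceType, and outputs it as spawned actors.
; Tick fills the matching capped counter through delay-gated macros and sphere-traces the output point, ignoring pipes, to detect blockage.
; AnyDamage triggers output: if unblocked, it spawns one stored item, throttled by a DoOnce and delay.
; A looping timer re-rolls Productivity by MachineLevel, though mining here uses a fixed delay.
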(event `self.ReceiveActorBeginOverlap`
  (params (OtherActor :type "Actor Object Reference")))

(event `self.ReceiveBeginPlay`
  (`parent.ReceiveBeginPlay`)
  (`self.ProductivityFix`)
  (`KismetSystemLibrary.K2_SetTimer` null "ProductivityFix" 15.0 true))

(event `self.ReceiveTick`
  (params (DeltaSeconds :type "Float (single-precision)"))
  (bind _returnvalue (`SceneComponent.K2_GetComponentLocation` (`self.Output_Point`)))
  (`parent.ReceiveTick` DeltaSeconds)
  (`|ExecutionSequence`
    (:`then_0`
      (switch `/Game/object_transform/E_Resourceİnfo` (`self.ResourceType`)
        (:`NewEnumerator0`
          (`self.MiningRawIron` 0.2))
        (:`NewEnumerator4`
          (`self.MiningCarbon` 0.2))
        (:`NewEnumerator2`
          (`self.MiningSoil` 0.2))))
    (:`then_1`
      (bind _outactors (`GameplayStatics.GetAllActorsOfClass` "/Game/object_transform/pipes/BP_Pipe.BP_Pipe_C"))
      (bind (_outhit _returnvalue_2) (`KismetSystemLibrary.SphereTraceSingle` _returnvalue _returnvalue 10.0 "TraceTypeQuery1" false _outactors "ForOneFrame"))
      (set `self.Is_Front_Emty` _returnvalue_2))))

(event `self.ReceiveAnyDamage`
  (params (Damage :type "Float (single-precision)") (DamageType :type "DamageType Object Reference") (InstigatedBy :type "Controller Object Reference") (DamageCauser :type "Actor Object Reference"))
  (`/Engine/EditorBlueprintResources/StandardMacros.DoOnce` false :!label _label
    (:`Completed`
      (`|ExecutionSequence`
        (:`then_0`
          (if (not (`self.Is_Front_Emty`))
            (switch `/Game/object_transform/E_Resourceİnfo` (`self.ResourceType`)
              (:`NewEnumerator0`
                (`self.RawIronSpawn`))
              (:`NewEnumerator4`
                (`self.CarbonSpawn`))
              (:`NewEnumerator2`
                (`self.SoilSpawn`)))))
        (:`then_1`
          (`KismetSystemLibrary.Delay` 0.2)
          (goto _label :!via `Reset`))))))

(fn `ProductivityFix`
  (bind _machinelevel (`self.MachineLevel`))
  (if (== _machinelevel 1)
    (set `self.Productivity` (`KismetMathLibrary.RandomFloatInRange` 3.0 4.0))
    (elif (== _machinelevel 2)
      (set `self.Productivity` (`KismetMathLibrary.RandomFloatInRange` 2.0 3.0))
      (elif (== _machinelevel 3)
        (set `self.Productivity` (`KismetMathLibrary.RandomFloatInRange` 1.0 2.0))
        (else
          (set `self.Productivity` (`KismetMathLibrary.RandomFloatInRange` 0.0 1.0)))))))

(fn `UserConstructionScript`
  (`parent.UserConstructionScript`))
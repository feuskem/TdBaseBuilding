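; Mold machine building that consumes overlapping Melt actors and converts their count into Plate or Capsule stock, as set by ResourceType.
; Each conversion is throttled by a Productivity delay, re-rolled every 15 seconds within a range set by MachineLevel.
; A per-tick sphere trace checks whether the output point is blocked, ignoring pipes.
; Damage ejects a stocked Plate when clear, with a short cooldown; the Capsule spawn function is not called here.
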(event `self.ReceiveBeginPlay`
  (`parent.ReceiveBeginPlay`)
  (`self.ProductivityFunction_Fix`)
  (`KismetSystemLibrary.K2_SetTimer` null "ProductivityFunction_Fix" 15.0 true))

(event `self.ReceiveTick`
  (params (DeltaSeconds :type "Float (single-precision)"))
  (bind _productivity (`self.Productivity`))
  (bind _returnvalue (`SceneComponent.K2_GetComponentLocation` (`self.Output_Point`)))
  (`parent.ReceiveTick` DeltaSeconds)
  (`|ExecutionSequence`
    (:`then_0`
      (for _array_element (`PrimitiveComponent.GetOverlappingActors` (`self.Box`) "/Game/object_transform/resources/melt.Melt_C")
        (`self.K2_DestroyActor` _array_element)
        (set `self.MeltMold` (+ (`self.MeltMold`) 1))))
    (:`then_1`
      (switch `/Game/object_transform/E_Resourceİnfo` (`self.ResourceType`)
        (:`NewEnumerator9`
          (`self.Plate` _productivity))
        (:`NewEnumerator10`
          (`self.Capsule` _productivity))))
    (:`then_2`
      (bind _outactors (`GameplayStatics.GetAllActorsOfClass` "/Game/object_transform/pipes/BP_Pipe.BP_Pipe_C"))
      (bind (_outhit _returnvalue_2) (`KismetSystemLibrary.SphereTraceSingle` _returnvalue _returnvalue 10.0 "TraceTypeQuery1" false _outactors "ForOneFrame"))
      (set `self.Hit` _returnvalue_2))))

(event `self.ReceiveAnyDamage`
  (params (Damage :type "Float (single-precision)") (DamageType :type "DamageType Object Reference") (InstigatedBy :type "Controller Object Reference") (DamageCauser :type "Actor Object Reference"))
  (`/Engine/EditorBlueprintResources/StandardMacros.DoOnce` false :!label _label
    (:`Completed`
      (`|ExecutionSequence`
        (:`then_0`
          (if (not (`self.Hit`))
            (switch `/Game/object_transform/E_Resourceİnfo` (`self.ResourceType`)
              (:`NewEnumerator9`
                (`self.SpawnPlate`)))))
        (:`then_1`
          (`KismetSystemLibrary.Delay` 0.2)
          (goto _label :!via `Reset`))))))

(fn `ProductivityFunction_Fix`
  (bind _machinelevel (`self.MachineLevel`))
  (if (== _machinelevel 1)
    (set `self.Productivity` (`KismetMathLibrary.RandomFloatInRange` 3.0 4.0))
    (elif (== _machinelevel 2)
      (set `self.Productivity` (`KismetMathLibrary.RandomFloatInRange` 2.0 3.0))
      (elif (== _machinelevel 3)
        (set `self.Productivity` (`KismetMathLibrary.RandomFloatInRange` 1.0 2.0))
        (else
          (set `self.Productivity` (`KismetMathLibrary.RandomFloatInRange` 0.0 1.0)))))))

(fn `UserConstructionScript`
  (`parent.UserConstructionScript`))
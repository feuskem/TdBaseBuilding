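; Energy Concentrator building that turns hydrogen and capsule items into stored Light Batteries.
; Tick absorbs items overlapping its box into counters and, in Light Battery mode, runs a timed conversion capped by storage.
; Conversion delay is rerolled periodically within ranges set by machine level.
; A sphere trace flags output blockage; damage checks it but reaches an empty resource switch, leaving the LightBatterySpawn macro uncalled.
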(event `self.ReceiveActorBeginOverlap`
  (params (OtherActor :type "Actor Object Reference"))
  (cast `/Game/Td/BP_Destroyer` OtherActor)
  (set `self.NewVar_0` "NewEnumerator7"))

(event `self.ReceiveBeginPlay`
  (`self.ProductivityFix`)
  (`KismetSystemLibrary.K2_SetTimer` null "ProductivityFix" 15.0 true))

(event `self.ReceiveTick`
  (params (DeltaSeconds :type "Float (single-precision)"))
  (bind _returnvalue (`SceneComponent.K2_GetComponentLocation` (`self.Output_Point`)))
  (`|ExecutionSequence`
    (:`then_0`
      (for _array_element (`PrimitiveComponent.GetOverlappingActors` (`self.Box`) "/Game/object_transform/resources/Hidrojen.Hidrojen_C")
        (`self.K2_DestroyActor` _array_element)
        (set `self.HidrojenEC` (+ (`self.HidrojenEC`) 1))))
    (:`then_1`
      (for _array_element_2 (`PrimitiveComponent.GetOverlappingActors` (`self.Box`) "/Game/object_transform/resources/Capsüle.Capsüle_C")
        (`self.K2_DestroyActor` _array_element_2)
        (set `self.CapsuleEC` (+ (`self.CapsuleEC`) 1))))
    (:`then_2`
      (switch `/Game/object_transform/E_Resourceİnfo` (`self.ResourceType`)
        (:`NewEnumerator12`
          (`self.LightBattery` (`self.Productivity`)))))
    (:`then_3`
      (bind _outactors (`GameplayStatics.GetAllActorsOfClass` "/Game/object_transform/pipes/BP_Pipe.BP_Pipe_C"))
      (bind (_outhit _returnvalue_2) (`KismetSystemLibrary.SphereTraceSingle` _returnvalue _returnvalue 10.0 "TraceTypeQuery1" false _outactors "ForOneFrame"))
      (set `self.Front` _returnvalue_2))))

(event `self.ReceiveAnyDamage`
  (params (Damage :type "Float (single-precision)") (DamageType :type "DamageType Object Reference") (InstigatedBy :type "Controller Object Reference") (DamageCauser :type "Actor Object Reference"))
  (`/Engine/EditorBlueprintResources/StandardMacros.DoOnce` false :!label _label
    (:`Completed`
      (`|ExecutionSequence`
        (:`then_0`
          (if (not (`self.Front`))
            (switch `/Game/object_transform/E_Resourceİnfo` (`self.ResourceType`))))
        (:`then_1`
          (`KismetSystemLibrary.Delay` 0.2)
          (goto _label :!via `Reset`))))))

(fn `ProductivityFix`
  (bind _machinelevel (`self.MachineLevel`))
  (if (== _machinelevel 1)
    (set `self.Productivity` (`KismetMathLibrary.RandomFloatInRange` 3.0 4.0))
    (elif (== _machinelevel 2)
      (set `self.Productivity` (`KismetMathLibrary.RandomFloatInRange` 2.0 3.0))
      (elif (== _machinelevel 3)
        (set `self.Productivity` (`KismetMathLibrary.RandomFloatInRange` 1.0 2.0))
        (else
          (set `self.Productivity` (`KismetMathLibrary.RandomFloatInRange` 0.0 1.0)))))))

(fn `UserConstructionScript`
  (`parent.UserConstructionScript`))
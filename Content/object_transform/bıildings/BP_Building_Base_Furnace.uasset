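; Furnace building that consumes overlapping Raw and Soil actors at its back box and converts them into stocks of melted iron or glass.
; Tick switches mode to the last input taken, runs delay-gated conversion macros and toggles furnace visuals from iron stock.
; Conversion delay is a level-based random value, re-rolled on a looping timer.
; AnyDamage serves as the output trigger, spawning one product when a sphere trace finds the output point clear.
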(event `self.ReceiveBeginPlay`
  (`parent.ReceiveBeginPlay`)
  (`self.ProductivityFunction_Fix`)
  (`KismetSystemLibrary.K2_SetTimer` null "ProductivityFunction_Fix" 15.0 true))

(event `self.ReceiveActorBeginOverlap`
  (params (OtherActor :type "Actor Object Reference"))
  (cast `/Game/Td/BP_Destroyer` OtherActor)
  (set `self.NewVar_0` "NewEnumerator1"))

(event `FurnanceUpdate`
  (if (or (!= (`self.Iron_Raw_Furnace`) 0) (!= (`self.Iron_Melt_Furnace`) 0))
    (`SceneComponent.SetHiddenInGame` (`self.PS_Furnance`) true false)
    (`SceneComponent.SetHiddenInGame` (`self.PaperFlipbook`) false false)
    (else
      (`SceneComponent.SetHiddenInGame` (`self.PS_Furnance`) false false)
      (`SceneComponent.SetHiddenInGame` (`self.PaperFlipbook`) true false))))

(event `self.ReceiveTick`
  (params (DeltaSeconds :type "Float (single-precision)"))
  (bind _backbox1 (`self.backBox1`))
  (bind _productivity (`self.Productivity`))
  (bind _returnvalue (`SceneComponent.K2_GetComponentLocation` (`self.Output_Point`)))
  (`parent.ReceiveTick` DeltaSeconds)
  (`self.FurnanceUpdate`)
  (`|ExecutionSequence`
    (:`then_0`
      (for _array_element (`PrimitiveComponent.GetOverlappingActors` _backbox1 "/Game/object_transform/resources/Raw.Raw_C")
        (`self.K2_DestroyActor` _array_element)
        (set `self.Iron_Raw_Furnace` (+ (`self.Iron_Raw_Furnace`) 1))
        (set `self.ResourceType` "NewEnumerator1")))
    (:`then_1`
      (for _array_element_2 (`PrimitiveComponent.GetOverlappingActors` _backbox1 "/Game/object_transform/resources/Soil.Soil_C")
        (`self.K2_DestroyActor` _array_element_2)
        (set `self.Soil_Furnace` (+ (`self.Soil_Furnace`) 1))
        (set `self.ResourceType` "NewEnumerator3")))
    (:`then_2`
      (switch `/Game/object_transform/E_Resourceİnfo` (`self.ResourceType`)
        (:`NewEnumerator1`
          (`self.MeltIron` _productivity))
        (:`NewEnumerator3`
          (`self.Glass` _productivity))))
    (:`then_3`
      (bind _outactors (`GameplayStatics.GetAllActorsOfClass` "/Game/object_transform/pipes/BP_Pipe.BP_Pipe_C"))
      (bind (_outhit _returnvalue_2) (`KismetSystemLibrary.SphereTraceSingle` _returnvalue _returnvalue 10.0 "TraceTypeQuery1" false _outactors "ForOneFrame"))
      (set `self.IsOverlap` _returnvalue_2))))

(event `self.ReceiveAnyDamage`
  (params (Damage :type "Float (single-precision)") (DamageType :type "DamageType Object Reference") (InstigatedBy :type "Controller Object Reference") (DamageCauser :type "Actor Object Reference"))
  (`/Engine/EditorBlueprintResources/StandardMacros.DoOnce` false :!label _label
    (:`Completed`
      (`|ExecutionSequence`
        (:`then_0`
          (if (not (`self.IsOverlap`))
            (switch `/Game/object_transform/E_Resourceİnfo` (`self.ResourceType`)
              (:`NewEnumerator1`
                (`self.SpawnMeltIron`))
              (:`NewEnumerator3`
                (`self.SpawnGlass`)))))
        (:`then_1`
          (`KismetSystemLibrary.Delay` 0.2)
          (goto _label :!via `Reset`))))))

(fn `ProductivityFunction_Fix`
  (bind _machinelevel (`self.MachineLevel`))
  (if (== _machinelevel 1)
    (set `self.Productivity` (`KismetMathLibrary.RandomFloatInRange` 3.0 4.0))
    (elif (== _machinelevel 2)
      (set `self.Productivity` (`KismetMathLibrary.RandomFloatInRange` 2.0 3.0))
      (elif (== _machinelevel 3)
        (set `self.Productivity` (`KismetMathLibrary.RandomFloatInRange` 1.0 2.0))
        (else
          (set `self.Productivity` (`KismetMathLibrary.RandomFloatInRange` 0.0 1.0)))))))

(fn `UserConstructionScript`
  (`parent.UserConstructionScript`))
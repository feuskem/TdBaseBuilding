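; Building Blueprint, apparently a constructor variant derived from a parent class, that takes in resource actors overlapping its Box.
; Each Tick runs the parent logic, then destroys overlapping Glass actors and increments Glass2Constractor per actor.
; A second pass also queries Glass, despite incrementing Plate2Constractor.
; A final switch on ResourceInfo has no connected cases, and BeginPlay and overlap events are disabled.
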(event `self.ReceiveTick`
  (params (DeltaSeconds :type "Float (single-precision)"))
  (`parent.ReceiveTick` DeltaSeconds)
  (`|ExecutionSequence`
    (:`then_0`
      (for _array_element (`PrimitiveComponent.GetOverlappingActors` (`self.Box`) "/Game/object_transform/resources/Glass.Glass_C")
        (`self.K2_DestroyActor` _array_element)
        (set `self.Glass_2Constractor` (+ (`self.Glass_2Constractor`) 1))))
    (:`then_1`
      (for _array_element_2 (`PrimitiveComponent.GetOverlappingActors` (`self.Box`) "/Game/object_transform/resources/Glass.Glass_C")
        (`self.K2_DestroyActor` _array_element_2)
        (set `self.Plate_2Constractor` (+ (`self.Plate_2Constractor`) 1))))
    (:`then_2`
      (switch `/Game/object_transform/E_Resourceİnfo` (`self.ResourceInfo`)))))

(fn `UserConstructionScript`
  (`parent.UserConstructionScript`))
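; Base miner building that produces raw iron and ejects it as mesh actors at its output point.
; Tick drives a DoOnce and Delay macro that adds one ore per second up to a small cap.
; Tick also sphere-traces at OutMiner, ignoring pipes, storing any hit in the misleadingly named IsFrontEmty.
; Receiving any damage spends one ore to spawn BP_Iron_Raw_Mesh there if nothing blocks it.
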(event `self.ReceiveTick`
  (params (DeltaSeconds :type "Float (single-precision)"))
  (bind _returnvalue (`SceneComponent.K2_GetComponentLocation` (`self.out_Miner`)))
  (`parent.ReceiveTick` 0.0)
  (`|ExecutionSequence`
    (:`then_0`
      (`self.Mining`))
    (:`then_1`
      (bind _outactors (`GameplayStatics.GetAllActorsOfClass` "/Game/object_transform/BP_Pipe.BP_Pipe_C"))
      (bind (_outhit _returnvalue_2) (`KismetSystemLibrary.SphereTraceSingle` _returnvalue _returnvalue 10.0 "TraceTypeQuery1" false _outactors "ForOneFrame"))
      (set `self.Is_Front_Emty` _returnvalue_2))))

(event `self.ReceiveAnyDamage`
  (params (Damage :type "Float (single-precision)") (DamageType :type "DamageType Object Reference") (InstigatedBy :type "Controller Object Reference") (DamageCauser :type "Actor Object Reference"))
  (bind _iron_raw_miner (`self.Iron Raw Miner`))
  (bind _out_miner (`self.out_Miner`))
  (if (`self.Is_Front_Emty`)
    _
    (elif (> _iron_raw_miner 0)
      (set `self.Iron Raw Miner` (- _iron_raw_miner 1))
      (`|SpawnActorFromClass` "/Game/object_transform/BP_Iron_Raw_Mesh.BP_Iron_Raw_Mesh_C" (`KismetMathLibrary.MakeTransform` (`SceneComponent.K2_GetComponentLocation` _out_miner) (`SceneComponent.K2_GetComponentRotation` _out_miner)) "Undefined" "OverrideRootScale" null null))))

(fn `UserConstructionScript`
  (`parent.UserConstructionScript`))
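; BP_Building_Base_Furnace is a furnace building that turns raw iron into melted iron.
; Overlapping raw iron meshes are destroyed after a short delay and added to a raw counter.
; Tick, gated by a resettable DoOnce and Delay, converts raw to melt one unit at a time up to a cap.
; AnyDamage serves as extraction, subtracting Damage from melt and spawning a melt mesh at OutFurnace, behind a DoOnce that is never reset.
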(event `self.ReceiveActorBeginOverlap`
  (params (OtherActor :type "Actor Object Reference"))
  (bind _asbp_iron_raw_mesh (cast `/Game/object_transform/BP_Iron_Raw_Mesh` OtherActor))
  (`KismetSystemLibrary.Delay` 0.5)
  (`self.K2_DestroyActor` _asbp_iron_raw_mesh)
  (set `self.Iron_Raw_Furnace` (+ (`self.Iron_Raw_Furnace`) 1)))

(event `self.ReceiveTick`
  (params (DeltaSeconds :type "Float (single-precision)"))
  (bind _iron_melt_furnace (`self.Iron_Melt_Furnace`))
  (`parent.ReceiveTick` DeltaSeconds)
  (`/Engine/EditorBlueprintResources/StandardMacros.DoOnce` false :!label _label
    (:`Completed`
      (if (> (`self.Iron_Raw_Furnace`) 0)
        (if (< _iron_melt_furnace 10)
          (bind _output_get (set `self.Iron_Melt_Furnace` (+ _iron_melt_furnace 1)))
          (set `self.Iron_Raw_Furnace` (- (`self.Iron_Raw_Furnace`) 1))
          (`KismetSystemLibrary.Delay` 1.0)
          (`KismetSystemLibrary.PrintString` (`KismetStringLibrary.Concat_StrStr` "melt " (`KismetStringLibrary.Conv_Int64ToString` _output_get)))
          (goto _label :!via `Reset`)
          (else
            (goto _label :!via `Reset`)))
        (else
          (goto _label :!via `Reset`))))))

(event `self.ReceiveAnyDamage`
  (params (Damage :type "Float (single-precision)") (DamageType :type "DamageType Object Reference") (InstigatedBy :type "Controller Object Reference") (DamageCauser :type "Actor Object Reference"))
  (bind _iron_melt_furnace (`self.Iron_Melt_Furnace`))
  (if (> _iron_melt_furnace 0)
    (`/Engine/EditorBlueprintResources/StandardMacros.DoOnce` false
      (:`Completed`
        (set `self.Iron_Melt_Furnace` (- _iron_melt_furnace Damage))
        (`|SpawnActorFromClass` "/Game/object_transform/BP_Iron_Melt_mesh.BP_Iron_Melt_mesh_C" (`KismetMathLibrary.MakeTransform` (`SceneComponent.K2_GetComponentLocation` (`self.out_Furnace`))) "Undefined" "OverrideRootScale" null null)))))

(fn `UserConstructionScript`
  (`parent.UserConstructionScript`))
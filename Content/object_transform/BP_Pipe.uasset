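; BP_Pipe is a pipe actor that uses damage events to act on the raw iron and buildings it overlaps.
; Each Tick runs two functions that gather overlapping BP_Building_Base and BP_Iron_Raw_Mesh actors.
; Each overlapped actor receives ApplyDamage scaled by delta time and a per-type rate, SpawnPerSecond for buildings and ResourceTouch for iron.
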(event `self.ReceiveBeginPlay`)

(event `self.ReceiveTick`
  (params (DeltaSeconds :type "Float (single-precision)"))
  (`|ExecutionSequence`
    (:`then_0`
      (`self.Stracture_Connection_Overlap` DeltaSeconds))
    (:`then_1`
      (`self.Base_Resources` DeltaSeconds))))

(fn `UserConstructionScript`)
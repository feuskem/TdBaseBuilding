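; BP_Pipe is a pipe actor that acts on the buildings and raw iron it overlaps through ApplyDamage calls.
; Each Tick, the Zort flag either switches off its collision, or leaves it on and runs two overlap passes.
; The passes damage BP_Building_Base actors by SpawnPerSecond and Iron_raw actors by ResourceTouch, both scaled by delta time.
; A PlayerController cast for placement mode is left unconnected.
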(event `self.ReceiveBeginPlay`)

(event `self.ReceiveTick`
  (params (DeltaSeconds :type "Float (single-precision)"))
  (if (`self.Zort`)
    (`self.SetActorEnableCollision` false)
    (else
      (`self.SetActorEnableCollision` true)
      (`|ExecutionSequence`
        (:`then_0`
          (`self.Stracture_Connection_Overlap` DeltaSeconds))
        (:`then_1`
          (`self.Base_Resources` DeltaSeconds))))))

(fn `UserConstructionScript`)
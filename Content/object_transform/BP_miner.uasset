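; BP_miner is a mining machine that produces raw iron and feeds it out to pipes.
; Tick adds one IronRaw per frame to the player controller's BP_collection while below 100, through a DoOnce that immediately resets.
; A BP_Pipe overlapping Output starts a three-second timer, looping per OutputOverlap, that spawns an iron mesh above Output without deducting from the count.
; End overlap clears that flag but not the timer.
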(event `self.ReceiveBeginPlay`
  (bind _asbp_collection (cast `/Game/object_transform/BP_collection` (`GameplayStatics.GetPlayerController` 0)))
  (set `self.As BP Collection` _asbp_collection)
  (`GameplayStatics.GetAllActorsOfClass` "/Game/object_transform/BP_Pipe.BP_Pipe_C"))

(event `self.ReceiveTick`
  (params (DeltaSeconds :type "Float (single-precision)"))
  (bind _as_bp_collection (`self.As BP Collection`))
  (bind _iron_raw (`/Game/object_transform/BP_collection.Iron Raw` _as_bp_collection))
  (`/Engine/EditorBlueprintResources/StandardMacros.DoOnce` false :!label _label
    (:`Completed`
      (if (< _iron_raw 100)
        (set `/Game/object_transform/BP_collection.Iron Raw` (+ _iron_raw 1) _as_bp_collection)
        (goto _label :!via `Reset`)
        (else
          (goto _label :!via `Reset`))))))

(event `self.output.OnComponentBeginOverlap`
  (params (OverlappedComponent :type "PrimitiveComponent Object Reference") (OtherActor :type "Actor Object Reference") (OtherComp :type "PrimitiveComponent Object Reference") (OtherBodyIndex :type Integer) (bFromSweep :type Boolean) (SweepResult :type "HitResult Structure (by ref)"))
  (cast `/Game/object_transform/BP_Pipe` OtherActor)
  (`KismetSystemLibrary.K2_SetTimer` null "Output_Pipe_Overlap_Evnt" 3.0 (`self.Output_Overlap`)))

(event `self.output.OnComponentEndOverlap`
  (params (OverlappedComponent :type "PrimitiveComponent Object Reference") (OtherActor :type "Actor Object Reference") (OtherComp :type "PrimitiveComponent Object Reference") (OtherBodyIndex :type Integer))
  (cast `/Game/object_transform/BP_Pipe` OtherActor)
  (set `self.Output_Overlap` false))

(event `Output_Pipe_Overlap_Evnt`
  (bind (_returnvalue_x _returnvalue_y _returnvalue_z) (`KismetMathLibrary.BreakVector` (`SceneComponent.K2_GetComponentLocation` (`self.output`))))
  (`|SpawnActorFromClass` "/Game/object_transform/BP_Iron_Raw_Mesh.BP_Iron_Raw_Mesh_C" (`KismetMathLibrary.MakeTransform` (`KismetMathLibrary.MakeVector` _returnvalue_x _returnvalue_y (+ _returnvalue_z 80.0))) "Undefined" "OverrideRootScale" null null))

(fn `UserConstructionScript`)